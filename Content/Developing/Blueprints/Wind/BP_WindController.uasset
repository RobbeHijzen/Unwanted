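; BP_WindController periodically blows the player balloon (BP_PlayerBalloon) with timed gusts of wind in random directions.
; A looping interval timer starts each burst, picking one of the preset directions.
; During a burst, a near-zero looping timer acts as a per-frame tick until the duration ends.
; Each tick offsets the balloon's collision sphere without sweeping, scaled by delta time and inversely by radius, so bigger balloons drift slower.
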(event `self.ReceiveBeginPlay`
  ;[1 1 1] Comment
  (`KismetSystemLibrary.K2_SetTimerDelegate` (delegate `StartWindburst`) (`self.WindInterval`) true)
  (bind _returnvalue (`GameplayStatics.GetActorOfClass` "/Game/Developing/Blueprints/Character/BP_PlayerBalloon.BP_PlayerBalloon_C"))
  (set `self.TargetActor` _returnvalue))

(event `StartWindburst`
  ;[1 1 1] Comment
  (set `self.WindActive` true)
  (bind _result (`/Engine/EditorBlueprintResources/StandardMacros.DecrementInt` (`KismetArrayLibrary.Array_Length` (`self.PossibleWindDirections`)))
    (:`  `
      (set `self.WindDirection` (`|GetArrayItem` (`self.PossibleWindDirections`) (`KismetMathLibrary.RandomIntegerInRange` 0 _result)))
      ;[1 1 1] TODO: make function + make better : move balloon function
      (bind _returnvalue (`KismetSystemLibrary.K2_SetTimerDelegate` (delegate `ApplyForce`) 1e-05 true true))
      (`KismetSystemLibrary.Delay` (`self.WindDuration`))
      (set `self.WindActive` false)
      (`KismetSystemLibrary.K2_ClearAndInvalidateTimerHandle` _returnvalue))))

(event `ApplyForce`
  (bind __ballooncollision (`PlayerBalloon._BalloonCollision` (`self.TargetActor`)))
  ;[1 1 1] TODO: make function + make better : move balloon function
  (set `self.balloonRadius` (`SphereComponent.GetScaledSphereRadius` __ballooncollision))
  (`SceneComponent.K2_AddWorldOffset` __ballooncollision (* (* (* (`self.WindDirection`) (`self.WindStrength`)) (`GameplayStatics.GetWorldDeltaSeconds`)) (/ (`self.SpeedScale`) (`self.balloonRadius`))) false false))

(fn `UserConstructionScript`)