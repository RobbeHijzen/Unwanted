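; BP_Flames_Child is a child flame actor that acts as an intermittent fire, periodically switching itself off.
; On BeginPlay it runs the parent logic, then starts a looping timer on the MoveFire event.
; MoveFire disables the box collision and hides the fire sprite, then restores both after a delay.
; The same Delay variable sets both the timer interval and the off duration.
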(event `self.ReceiveBeginPlay`
  (`parent.ReceiveBeginPlay`)
  (`KismetSystemLibrary.K2_SetTimerDelegate` (delegate `move fire`) (`self.delay`) true))

(event `move fire`
  (bind _fire_sprite (`self.fire sprite`))
  (bind _box (`self.Box`))
  (`PrimitiveComponent.SetCollisionEnabled` _box "NoCollision")
  (`SceneComponent.SetHiddenInGame` _fire_sprite true false)
  (`KismetSystemLibrary.Delay` (`self.delay`))
  (`SceneComponent.SetHiddenInGame` _fire_sprite false false)
  (`PrimitiveComponent.SetCollisionEnabled` _box "QueryAndPhysics"))

(fn `UserConstructionScript`
  (`parent.UserConstructionScript`))