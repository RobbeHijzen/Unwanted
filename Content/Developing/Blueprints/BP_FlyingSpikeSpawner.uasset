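; BP_FlyingSpikeSpawner spawns flying spike birds at its location while the player balloon is within its active zone.
; Overlapping Box_Bot with BP_PlayerBalloon activates spawning, and overlapping Box_Top deactivates it.
; While active, Tick accumulates time toward a randomized interval, spawns BP_FlyingSpike_Child, then rerolls the interval.
; SpawningBirdsToLeft rotates spawned birds 180 degrees to reverse their heading.
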(event `self.ReceiveTick`
  (params (DeltaSeconds :type "Float (single-precision)"))
  (if (`self.PlayerInRange`)
    (bind _output_get (set `self.CurrentSpawningTime` (+ (`self.CurrentSpawningTime`) DeltaSeconds)))
    (if (>= _output_get (`self.CurrentRandomSpawningTime`))
      (`self.SpawnBird`)
      (set `self.CurrentSpawningTime` 0.0)
      (`self.CalculateRandomSpawningTime`))))

(event `self.Box_Bot.OnComponentBeginOverlap`
  (params (OverlappedComponent :type "PrimitiveComponent Object Reference") (OtherActor :type "Actor Object Reference") (OtherComp :type "PrimitiveComponent Object Reference") (OtherBodyIndex :type Integer) (bFromSweep :type Boolean) (SweepResult :type "HitResult Structure (by ref)"))
  (cast `/Game/Developing/Blueprints/Character/BP_PlayerBalloon` OtherActor)
  (set `self.PlayerInRange` true)
  (`self.CalculateRandomSpawningTime`))

(event `self.Box_Top.OnComponentBeginOverlap`
  (params (OverlappedComponent :type "PrimitiveComponent Object Reference") (OtherActor :type "Actor Object Reference") (OtherComp :type "PrimitiveComponent Object Reference") (OtherBodyIndex :type Integer) (bFromSweep :type Boolean) (SweepResult :type "HitResult Structure (by ref)"))
  (cast `/Game/Developing/Blueprints/Character/BP_PlayerBalloon` OtherActor)
  (set `self.PlayerInRange` false))

(event `CalculateRandomSpawningTime`
  (set `self.CurrentRandomSpawningTime` (`KismetMathLibrary.RandomFloatInRange` (`self.MinSpawningTime`) (`self.MaxSpawningTime`))))

(event `SpawnBird`
  (`|SpawnActorFromClass` "/Game/Developing/Blueprints/BP_FlyingSpike_Child.BP_FlyingSpike_Child_C" (`KismetMathLibrary.MakeTransform` (`self.K2_GetActorLocation`) (select `bool` (`self.SpawningBirdsToLeft`) :`false` (struct) :`true` (struct :`Yaw` 180.0) :!type "Rotator Structure")) "Undefined" "MultiplyWithRoot" null null))

(fn `UserConstructionScript`)