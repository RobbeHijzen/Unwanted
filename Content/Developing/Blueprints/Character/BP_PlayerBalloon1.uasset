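; Player balloon Blueprint that reacts to its size-changed and popped events, both bound on BeginPlay.
; Size changes scale the Balloon component by CurrentRadius relative to a base of 50 and set the physics constraint's linear Z limit to that radius.
; Popping enables physics simulation on BalloonCollision and copies its linear damping onto the Child component.
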(event `self.ReceiveBeginPlay`
  (add `self._OnPopped` (delegate `_OnPopped_Event`))
  (add `self._OnSizeChanged` (delegate `ResizeSphere`)))

(event `ResizeSphere`
  (`|ExecutionSequence`
    (:`then_0`
      (`SceneComponent.SetWorldScale3D` (`self.Balloon`) (`KismetMathLibrary.Conv_DoubleToVector` (/ (`self._CurrentRadius`) 50.0))))
    (:`then_1`
      (`PhysicsConstraintComponent.SetLinearZLimit` (`self.PhysicsConstraint`) "LCM_Limited" (`self._CurrentRadius`)))))

(event `_OnPopped_Event`
  (`PrimitiveComponent.SetSimulatePhysics` (`self._BalloonCollision`) true)
  (`PrimitiveComponent.SetLinearDamping` (`self.Child`) (`PrimitiveComponent.GetLinearDamping` (`self._BalloonCollision`))))

(fn `UserConstructionScript`)