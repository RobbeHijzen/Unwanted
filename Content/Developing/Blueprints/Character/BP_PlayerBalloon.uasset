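; Player balloon with a physics-constrained Child, animated with Paper2D flipbooks for idle, left/right movement and popping.
; Size-change events rescale the balloon and its constraint's Z limit; popping enables collision physics and locks Child to the YZ plane.
; Tick clamps horizontal position, lets the camera follow only vertically, and counter-tilts the balloon flipbook against the other flipbook's pitch, scaled by radius.
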(event `self.ReceiveBeginPlay`
  (add `self._OnStoppedMoving` (delegate `_OnStoppedMoving_Event`))
  (add `self._OnMovingToLeft` (delegate `_OnMovingToLeft_Event`))
  (add `self._OnMovingToRight` (delegate `_OnMovingToRight_Event`))
  (add `self._OnPopped` (delegate `_OnPopped_Event_0`))
  (add `self._OnSizeChanged` (delegate `ResizeSphere`))
  (set `self.BeginPositionCamera` (`SceneComponent.K2_GetComponentLocation` (`self.Camera`))))

(event `ResizeSphere`
  (`|ExecutionSequence`
    (:`then_0`
      (`SceneComponent.SetWorldScale3D` (`self.Balloon`) (`KismetMathLibrary.Conv_DoubleToVector` (/ (`self._CurrentRadius`) 50.0))))
    (:`then_1`
      (`PhysicsConstraintComponent.SetLinearZLimit` (`self.PhysicsConstraint`) "LCM_Limited" (* (`self._CurrentRadius`) 1.75)))))

(event `_OnStoppedMoving_Event`
  (`PaperFlipbookComponent.SetFlipbook` (`self.PaperFlipbook`) "/Game/Developing/Animations/Idle.Idle"))

(event `_OnMovingToLeft_Event`
  (`PaperFlipbookComponent.SetFlipbook` (`self.PaperFlipbook`) "/Game/Developing/Animations/MoveLeft.MoveLeft"))

(event `_OnPopped_Event_0`
  (bind _paperflipbook1 (`self.PaperFlipbook1`))
  (`|ExecutionSequence`
    (:`then_0`
      (`PrimitiveComponent.SetSimulatePhysics` (`self._BalloonCollision`) true)
      (`PrimitiveComponent.SetLinearDamping` (`self.Child`) (`PrimitiveComponent.GetLinearDamping` (`self._BalloonCollision`)))
      (`PaperFlipbookComponent.SetFlipbook` _paperflipbook1 "/Game/Developing/Animations/BalloonPOP.BalloonPOP")
      (`PaperFlipbookComponent.SetLooping` _paperflipbook1 false)
      (`KismetSystemLibrary.Delay` (`PaperFlipbookComponent.GetFlipbookLength` _paperflipbook1))
      (`PaperFlipbookComponent.SetFlipbook` _paperflipbook1 null))
    (:`then_1`
      (`PrimitiveComponent.SetConstraintMode` (`self.Child`) "YZPlane"))))

(event `_OnMovingToRight_Event`
  (`PaperFlipbookComponent.SetFlipbook` (`self.PaperFlipbook`) "/Game/Developing/Animations/MoveRight.MoveRight"))

(event `self.ReceiveTick`
  (params (DeltaSeconds :type "Float (single-precision)"))
  (bind (_beginpositioncamera_x _beginpositioncamera_y) (`KismetMathLibrary.BreakVector` (`self.BeginPositionCamera`)))
  (bind __boundswidth (`self._BoundsWidth`))
  (bind (_returnvalue_x _returnvalue_y _returnvalue_z) (`KismetMathLibrary.BreakVector` (`SceneComponent.K2_GetComponentLocation` (`self._BalloonCollision`))))
  (bind (_returnvalue_x_2 _returnvalue_y_2 _returnvalue_z_2) (`KismetMathLibrary.BreakVector` (`SceneComponent.K2_GetComponentLocation` (`self.Camera`))))
  (bind (_returnvalue_roll _returnvalue_pitch) (`KismetMathLibrary.BreakRotator` (`SceneComponent.K2_GetComponentRotation` (`self.PaperFlipbook`))))
  (bind (_returnvalue_x_3 _returnvalue_y_3 _returnvalue_z_3) (`KismetMathLibrary.BreakVector` (`SceneComponent.K2_GetComponentLocation` (`self._BalloonCollision`))))
  (bind _returnvalue (* (`self._BoundsWidth`) -1.0))
  (`|ExecutionSequence`
    (:`then_0`
      (if (> _returnvalue_x_3 __boundswidth)
        (`SceneComponent.K2_SetWorldLocation` (`self._BalloonCollision`) (`KismetMathLibrary.MakeVector` __boundswidth _returnvalue_y_3 _returnvalue_z_3) false false)))
    (:`then_1`
      (if (< _returnvalue_x _returnvalue)
        (`SceneComponent.K2_SetWorldLocation` (`self._BalloonCollision`) (`KismetMathLibrary.MakeVector` _returnvalue _returnvalue_y _returnvalue_z) false false)))
    (:`then_2`
      (`SceneComponent.K2_SetWorldLocation` (`self.Camera`) (`KismetMathLibrary.MakeVector` _beginpositioncamera_x _beginpositioncamera_y _returnvalue_z_2) false false)
      (`SceneComponent.K2_SetWorldRotation` (`self.PaperFlipbook1`) (`KismetMathLibrary.MakeRotator` 0.0 (* (* _returnvalue_pitch -1.0) (`KismetMathLibrary.FClamp` (/ (- (`self._CurrentRadius`) (`self._MinRadius`)) (- (`self._MaxRadius`) (`self._MinRadius`))) 0.2 0.85))) false false))))

(fn `UserConstructionScript`)